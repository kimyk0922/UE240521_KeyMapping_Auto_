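; Demo actor with a named cube that animates automatically on a Timeline from BeginPlay.
; BeginPlay sets and positions the text label from variables, then starts the Timeline at a random time so its phase varies.
; Each update drives the cube's relative X, the label color and the material's Base_Color parameter.
; A Timeline event track toggles label visibility through a FlipFlop.
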(event `self.ReceiveBeginPlay`
  ;[0.3482 0.5721 0.75 1 15] Text_Name_&&_Location_
  (`TextRenderComponent.K2_SetText` (`self.Cube name`) (`self.Box Name`))
  (`SceneComponent.K2_SetRelativeLocation` (`self.Cube name`) (`KismetMathLibrary.MakeVector` (`self.Text Location X`) (`self.Text Location Y`) (`self.Text Location Z`)) false false)
  ;[1 0.9146 0.602 1 15] Auto_Move_
  (`|ExecutionSequence`
    (:`then_0`
      (bind (_direction _time_line) (`Timeline|Timeline` :`NewTime` (`KismetMathLibrary.RandomFloatInRange` 0.0 1.0) :!via `SetNewTime` :!label _label)
        (:`Update`
          (`SceneComponent.K2_SetRelativeLocation` (`self.Cube`) (`KismetMathLibrary.MakeVector` (* _time_line 100.0)) false false)
          ;[1 0.633 0.6729 1 15] Text_Color_
          (`TextRenderComponent.SetTextRenderColor` (`self.Cube name`) (`self.Value`))
          ;[0.7708 0.5417 1 1 15] Meterial_Base_Color
          (`MeshComponent.SetVectorParameterValueOnMaterials` (`self.Cube`) "Base_Color" (`self.Meterial_Color`)))
        (:`TL_Event`
          ;[0.526 0.526 0.526 1 14] Text_Visibility_
          (bind _isa (`/Engine/EditorBlueprintResources/StandardMacros.FlipFlop`)
            (:`A`
              _)
            (:`B`
              _))
          (`SceneComponent.SetVisibility` (`self.Cube name`) _isa false))))
    (:`then_1`
      (goto _label))))

(fn `UserConstructionScript`)