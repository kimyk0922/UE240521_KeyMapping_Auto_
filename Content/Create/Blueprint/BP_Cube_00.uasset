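; BP_Cube_00 is an input-driven test actor whose cube steps upward each time the 1 key is pressed.
; BeginPlay enables input from the first player controller on the actor.
; Each press increments a counter that wraps to zero after ten and sets the cube's relative Z position from it in fixed steps.
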(event `self.ReceiveBeginPlay`
  ;[0.7052 1 0.715] Key_Mapping_Input_
  (`self.EnableInput` (`GameplayStatics.GetPlayerController` 0)))

(event `Key|One`
  (params (Key :type "Key Structure"))
  (bind _num (`self.Num`))
  (:`Pressed`
    ;[0.05448 0.1683 0.1274] Actor_Move_
    (set `self.Num` (+ _num 1))
    (if (> _num 10)
      (set `self.Num` 0))
    (`SceneComponent.K2_SetRelativeLocation` (`self.Cube`) (`KismetMathLibrary.MakeVector` 0.0 0.0 (* (`self.Num`) 100)) false false)))

(fn `UserConstructionScript`)